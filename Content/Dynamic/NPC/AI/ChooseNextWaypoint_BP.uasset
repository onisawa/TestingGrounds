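; Behavior tree task that picks the next patrol waypoint for an AI-controlled NPC.
; It reads the PatrolPoints array from the controlled pawn, then writes the point at the Blackboard Index to the WayPoint key.
; It then increments Index with a modulo wrap so the patrol loops, and finishes successfully.
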(event EventReceiveExecuteAI
  (params (OwnerController :type AI%20Controller%20Object%20Reference) (ControlledPawn :type Pawn%20Object%20Reference))
  (CallFunction|GetPatrolPoint ControlledPawn)
  (bind _index (CallFunction|SetNextWaypoint))
  (CallFunction|CycleIndex _index)
  (AI|BehaviorTree|FinishExecute true))

(fn GetPatrolPoint
  (params (Object :type Object%20Object%20Reference))
  (bind _assoldier (Utilities|Casting|CastTo Object))
  (Variables|Default|SetPatrol%20Points (Variables|Default|GetPatrol%20Points _assoldier)))

(fn SetNextWaypoint
  (bind _index (Variables|Default|Getindex))
  (bind _returnvalue (Class|BTFunctionLibrary|GetBlackboardValueasInt _index))
  (Class|BTFunctionLibrary|SetBlackboardValueasObject (Variables|Default|GetWayPoint) (Utilities|Array|Get(acopy) (Variables|Default|GetPatrol%20Points) _returnvalue))
  (return _returnvalue))

(fn CycleIndex
  (params (Index :type Integer))
  (Class|BTFunctionLibrary|SetBlackboardValueasInt (Variables|Default|Getindex) (Math|Integer|%(Integer) (+ Index 1) (Utilities|Array|Length (Variables|Default|GetPatrol%20Points)))))